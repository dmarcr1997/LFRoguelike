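; Black hole projectile that applies radial force and destroys actors it hits.
; Tick fires a RadialForceComponent impulse every frame and runs into a latent delay that destroys the projectile about five seconds after its first tick.
; SphereComp hits destroy any actor other than the instigator, while sphere overlaps only print the other actor's name.
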(event `self.ReceiveTick`
  (params (DeltaSeconds :type "Float (single-precision)"))
  (`RadialForceComponent.FireImpulse` (`self.RadialForceComponent`))
  (`KismetSystemLibrary.Delay` 5.0)
  (`self.K2_DestroyActor`))

(event `self.SphereComp.OnComponentBeginOverlap`
  (params (OverlappedComponent :type "PrimitiveComponent Object Reference") (OtherActor :type "Actor Object Reference") (OtherComp :type "PrimitiveComponent Object Reference") (OtherBodyIndex :type Integer) (bFromSweep :type Boolean) (SweepResult :type "HitResult Structure (by ref)"))
  (`KismetSystemLibrary.PrintText` (`KismetTextLibrary.Conv_StringToText` (`KismetSystemLibrary.GetDisplayName` OtherActor))))

(event `self.SphereComp.OnComponentHit`
  (params (HitComponent :type "PrimitiveComponent Object Reference") (OtherActor :type "Actor Object Reference") (OtherComp :type "PrimitiveComponent Object Reference") (NormalImpulse :type "Vector Structure") (Hit :type "HitResult Structure (by ref)"))
  (if (!= OtherActor (`self.GetInstigator`))
    (`self.K2_DestroyActor` OtherActor)))

(fn `UserConstructionScript`)